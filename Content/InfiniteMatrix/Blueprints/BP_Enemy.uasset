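; Enemy actor that hurts the player on contact and awards score when shot.
; A Box overlap casts the other actor to BP_Player or BP_Projectile to choose the response.
; Player contact calls ProcessHit, plays a sound and world camera shake, then destroys the enemy.
; A projectile hit plays a sound, increments Score through PlayerReference, then destroys both projectile and enemy.
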(event `self.ReceiveActorBeginOverlap`
  (params (OtherActor :type "Actor Object Reference")))

(event `self.Box.OnComponentBeginOverlap`
  (params (OverlappedComponent :type "PrimitiveComponent Object Reference") (OtherActor :type "Actor Object Reference") (OtherComp :type "PrimitiveComponent Object Reference") (OtherBodyIndex :type Integer) (bFromSweep :type Boolean) (SweepResult :type "HitResult Structure (by ref)"))
  (bind _playerreference (`self.PlayerReference`))
  (bind _asbp_player (cast `/Game/InfiniteMatrix/Blueprints/BP_Player` OtherActor)
    (:`then`
      (`/Game/InfiniteMatrix/Blueprints/BP_Player.ProcessHit` _asbp_player 0.5)
      (`GameplayStatics.PlaySound2D` "/Game/InfiniteMatrix/Audio/power-down-42676.power-down-42676" 1.0 1.0 0.0 null null)
      (`GameplayStatics.PlayWorldCameraShake` "/Game/InfiniteMatrix/Blueprints/BP_CameraShake.BP_CameraShake_C" (`self.K2_GetActorLocation` (`GameplayStatics.GetPlayerPawn` 0)) 0.0 750.0))
    (:`CastFailed`
      (bind _asbp_projectile (cast `/Game/InfiniteMatrix/Blueprints/BP_Projectile` OtherActor))
      (`GameplayStatics.PlaySound2D` "/Game/InfiniteMatrix/Audio/laser-zap-90575.laser-zap-90575" 1.0 1.0 0.0 null null)
      (set `/Game/InfiniteMatrix/Blueprints/BP_Player.Score` (+ (`/Game/InfiniteMatrix/Blueprints/BP_Player.Score` _playerreference) 1) _playerreference)
      (`/Engine/EditorBlueprintResources/StandardMacros.IsValid` _asbp_projectile
        (:`Is Valid`
          (`self.K2_DestroyActor` _asbp_projectile)))))
  (`/Engine/EditorBlueprintResources/StandardMacros.IsValid` self
    (:`Is Valid`
      (`self.K2_DestroyActor`))))

(fn `UserConstructionScript`)